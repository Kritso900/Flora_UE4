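; Player character with movement and look input that lets the player pick up, rotate and place MediumActor_BP objects on a grid.
; Tick line-traces from the camera to an arrow, snapping hits on Grid or GridExtender_BP to 8-unit steps and easing a spawned pointer toward them.
; A gate makes the held object follow the pointer, tinting its indicator by a box-overlap check.
; Interact picks up objects under the pointer or places them when unblocked.
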(event `InputAxis|MoveUp`
  (params (AxisValue :type "Float (single-precision)"))
  (`self.AddMovementInput` (`self.GetActorForwardVector`) AxisValue))

(event `InputAxis|MoveRight`
  (params (AxisValue :type "Float (single-precision)"))
  (`self.AddMovementInput` (`self.GetActorRightVector`) AxisValue))

(event `self.ReceiveBeginPlay`
  (bind _returnvalue (`|SpawnActorFromClass` "/Game/MoveableObjects/ObjectPointer.ObjectPointer_C" (`KismetMathLibrary.MakeTransform` (0.0 0.0 0.0)) "Undefined" "OverrideRootScale" null null)))

(event `InputAxis|LookRight`
  (params (AxisValue :type "Float (single-precision)"))
  (`self.AddControllerYawInput` AxisValue))

(event `InputAxis|LookUp`
  (params (AxisValue :type "Float (single-precision)"))
  (`self.AddControllerPitchInput` (* AxisValue -1.0)))

(event `self.ReceiveTick`
  (params (DeltaSeconds :type "Float (single-precision)"))
  (bind _held_object_reference (`self.Held Object Reference`))
  (set `self.Delta Seconds` DeltaSeconds)
  (`|ExecutionSequence`
    (:`then_0`
      (`SceneComponent.K2_SetWorldTransform` (`Actor.RootComponent` (stale `self.ReceiveBeginPlay` _returnvalue)) (`KismetMathLibrary.TInterpTo` (`SceneComponent.K2_GetComponentToWorld` (`Actor.RootComponent` (stale `self.ReceiveBeginPlay` _returnvalue))) (stale _output_get) (`self.Delta Seconds`) 6.0) false false)
      (`KismetSystemLibrary.Delay` 0.1)
      (bind (_outhit _returnvalue) (`KismetSystemLibrary.LineTraceSingleForObjects` (`SceneComponent.K2_GetComponentLocation` (`self.Camera`)) (`SceneComponent.K2_GetComponentLocation` (`self.Arrow1`)) (`self.GridObjectType`)))
      (if _returnvalue
        (bind (_bblockinghit _binitialoverlap _time _distance _location _impactpoint _normal _impactnormal _physmat _hitactor) (`GameplayStatics.BreakHitResult` _outhit))
        (cast `/Game/MoveableObjects/Grid` _hitactor
          (:`then`
            (bind _output_get (set `self.NewVar_0` (`KismetMathLibrary.MakeTransform` (`KismetMathLibrary.MakeVector` (* (`KismetMathLibrary.Round` (/ (.x _location) 8.0)) 8.0) (* (`KismetMathLibrary.Round` (/ (.y _location) 8.0)) 8.0) (.z _location)))))
            (set `self.Is Player looking at a valid grid` true :!label _label))
          (:`CastFailed`
            (cast `/Game/MoveableObjects/GridExtender_BP` _hitactor
              (:`then`
                (goto _label))
              (:`CastFailed`
                (set `self.Is Player looking at a valid grid` false)))))
        (else
          (set `self.Is Player looking at a valid grid` false))))
    (:`then_1`
      (`/Engine/EditorBlueprintResources/StandardMacros.Gate` true :!label _label_2
        (:`Exit`
          (bind _returnvalue_2 (`KismetMathLibrary.VInterpTo` (`self.K2_GetActorLocation` (stale `InputAction|Interact` _output_get)) (`self.K2_GetActorLocation` (stale `self.ReceiveBeginPlay` _returnvalue)) (`self.Delta Seconds`) 8.0))
          (`self.K2_SetActorLocation` (stale `InputAction|Interact` _output_get) (`KismetMathLibrary.MakeVector` (.x _returnvalue_2) (.y _returnvalue_2) (+ (.z _returnvalue_2) 1.0)) false false)
          (bind _asmedium_actor_bp (cast `/Game/MoveableObjects/MediumActor_BP` _held_object_reference))
          (bind _boxextent (`BoxComponent.BoxExtent` (`/Game/MoveableObjects/MediumActor_BP.Collision Box` _asmedium_actor_bp)))
          (bind (_outactors _returnvalue_3) (`KismetSystemLibrary.BoxOverlapActors` (`KismetMathLibrary.MakeVector` (.x _returnvalue_2) (.y _returnvalue_2) (+ (.z _returnvalue_2) (.z _boxextent))) _boxextent (`self.Placedown blocker Object Types`) null (`|MakeArray` _held_object_reference)))
          (if _returnvalue_3
            (bind _collision_indicator (`/Game/MoveableObjects/MediumActor_BP.Collision Indicator` _asmedium_actor_bp))
            (`PrimitiveComponent.SetMaterial` _collision_indicator 0 "/Game/MoveableObjects/CollisionBAD_M.CollisionBAD_M")
            (else
              (`PrimitiveComponent.SetMaterial` _collision_indicator 0 "/Game/MoveableObjects/CollisionOK_M.CollisionOK_M"))))))))

(event `InputAction|Interact`
  (params (Key :type "Key Structure"))
  (bind _held_object_reference (`self.Held Object Reference`))
  (:`Pressed`
    (if (`self.Is Player looking at a valid grid`)
      (if (`self.Is holding object`)
        (bind _asmedium_actor_bp (cast `/Game/MoveableObjects/MediumActor_BP` _held_object_reference))
        (bind _returnvalue (`KismetMathLibrary.MakeVector` (* (`KismetMathLibrary.Round` (/ (.x (`.Location` (`GameplayStatics.BreakHitResult` (stale `self.ReceiveTick` _outhit)))) 8.0)) 8.0) (* (`KismetMathLibrary.Round` (/ (.y (`.Location` (`GameplayStatics.BreakHitResult` (stale `self.ReceiveTick` _outhit)))) 8.0)) 8.0) (.z (`.Location` (`GameplayStatics.BreakHitResult` (stale `self.ReceiveTick` _outhit))))))
        (bind _boxextent (`BoxComponent.BoxExtent` (`/Game/MoveableObjects/MediumActor_BP.Collision Box` _asmedium_actor_bp)))
        (bind (_outactors _returnvalue_2) (`KismetSystemLibrary.BoxOverlapActors` (`KismetMathLibrary.MakeVector` (.x _returnvalue) (.y _returnvalue) (+ (.z _returnvalue) (.z _boxextent))) _boxextent (`self.Placedown blocker Object Types`) null (`|MakeArray` _held_object_reference)))
        (if (not _returnvalue_2)
          (`|ExecutionSequence`
            (:`then_0`
              (goto _label_2 :!via `Close`))
            (:`then_1`
              (set `self.Is holding object` false) ; If the player is holding an object, looking \nat a valid placement location, and the \nobject isn't overlaping another object or a wall \nthen pressing interact will place the object down
              (`/Game/MoveableObjects/MediumActor_BP.Place Object_Event` _asmedium_actor_bp _returnvalue) ; Tells the object it is being placed down
            )))
        (else
          (bind (_outactors_2 _returnvalue_3) (`KismetSystemLibrary.BoxOverlapActors` (`SceneComponent.K2_GetComponentLocation` (`/Game/MoveableObjects/ObjectPointer.Cube` (stale `self.ReceiveBeginPlay` _returnvalue))) (1.0 1.0 20.0) (`self.Pickup-able Object Types`)))
          (if _returnvalue_3
            (bind _output_get (set `self.Held Object Reference` (`|GetArrayItem` _outactors_2)))
            (bind _asmedium_actor_bp_2 (cast `/Game/MoveableObjects/MediumActor_BP` (`self.Held Object Reference`)))
            (`/Game/MoveableObjects/MediumActor_BP.Pickup Object_Event` _asmedium_actor_bp_2)
            (set `self.Is holding object` true)
            (goto _label_2 :!via `Open`)))))))

(event `InputAction|RotateLeft`
  (params (Key :type "Key Structure"))
  (:`Pressed`
    (if (`self.Is Holding Object`)
      (bind _asmedium_actor_bp (cast `/Game/MoveableObjects/MediumActor_BP` (`self.Held Object Reference`)))
      (`/Game/MoveableObjects/MediumActor_BP.Rotate Left` _asmedium_actor_bp))))

(event `InputAction|RotateRight`
  (params (Key :type "Key Structure"))
  (:`Pressed`
    (if (`self.Is Holding Object`)
      (bind _asmedium_actor_bp (cast `/Game/MoveableObjects/MediumActor_BP` (`self.Held Object Reference`)))
      (`/Game/MoveableObjects/MediumActor_BP.Rotate Right` _asmedium_actor_bp))))

(fn `UserConstructionScript`)