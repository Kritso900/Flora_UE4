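; Moveable object actor that can be picked up, rotated and placed.
; A size enum selects the collision indicator scale and box extent on BeginPlay.
; Bound pickup and place events toggle held state and box collision, while rotate events cycle through four target rotations only while held.
; Tick eases the actor to its placement location when not held and always interpolates toward the target rotation.
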(event `self.ReceiveBeginPlay`
  (add `self.Place Object` (delegate `Place Object_Event`))
  (add `self.Pickup Object` (delegate `Pickup Object_Event`))
  (add `self.Rotate Left` (delegate `Rotate Left_Event`))
  (add `self.Rotate Right` (delegate `Rotate Right_Event`))
  (set `self.Object is Held` false)
  (set `self.Placement Location` (`self.K2_GetActorLocation`))
  (switch `/Game/EnvironmentArt/MoveableObjects/ObjectScale_ENum` (`self.Object scale ENum`)
    (:`NewEnumerator0`
      (set `self.Object Scale` 1))
    (:`NewEnumerator1`
      (set `self.Object Scale` 2))
    (:`NewEnumerator2`
      (set `self.Object Scale` 3)))
  (`SceneComponent.SetWorldScale3D` (`self.Collision Indicator`) (`BlueprintMapLibrary.Map_Find` (`self.Collision checker Scale`) (`self.Object Scale`)))
  (`BoxComponent.SetBoxExtent` (`self.Collision Box`) (`BlueprintMapLibrary.Map_Find` (`self.Collision box Scale`) (`self.Object Scale`)) false))

(event `Place Object_Event` :!signature `self.Place Object`
  (params (`Placement Location` :type "Vector Structure"))
  (set `self.Placement Location` `Placement Location`)
  (`PrimitiveComponent.SetCollisionEnabled` (`self.Collision Box`) "QueryAndPhysics")
  (set `self.Object is Held` false))

(event `self.ReceiveTick`
  (params (DeltaSeconds :type "Float (single-precision)"))
  (`|ExecutionSequence`
    (:`then_0`
      (if (not (`self.Object is Held`))
        (`self.K2_SetActorLocation` (`KismetMathLibrary.VInterpTo` (`self.K2_GetActorLocation`) (`self.Placement Location`) DeltaSeconds 12.0))))
    (:`then_1`
      (`self.K2_SetActorRotation` (`KismetMathLibrary.RInterpTo` (`self.K2_GetActorRotation`) (`|GetArrayItem` (`self.Rotations`) (`self.Target Rotation`)) DeltaSeconds 5.0)))))

(event `Pickup Object_Event`
  (`PrimitiveComponent.SetCollisionEnabled` (`self.Collision Box`) "NoCollision")
  (set `self.Object is Held` true))

(event `Rotate Left_Event`
  (bind _target_rotation (`self.Target Rotation`))
  (if (`self.Object is Held`)
    (if (== _target_rotation 0)
      (set `self.Target Rotation` 3)
      (else
        (`/Engine/EditorBlueprintResources/StandardMacros.DecrementInt` _target_rotation)))))

(event `Rotate Right_Event`
  (bind _target_rotation (`self.Target Rotation`))
  (if (`self.Object is Held`)
    (if (== _target_rotation 3)
      (set `self.Target Rotation` 0)
      (else
        (`/Engine/EditorBlueprintResources/StandardMacros.IncrementInt` _target_rotation)))))

(fn `UserConstructionScript`)