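; ObjectPointer_BP is an unfinished pointer actor, apparently meant for picking up and moving plant objects.
; BeginPlay binds an interact-press event, but that handler is empty.
; Tick runs a gated location interpolation whose target is the actor's current location, so it moves nothing.
; Disconnected logic sketches a hold/release toggle and a box overlap plant check that only prints, with grid snapping noted as a TODO.
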(event `self.ReceiveBeginPlay`
  (add `self.Interact pressed` (delegate `Interact pressed_Event`)))

(event `Interact pressed_Event`)

(event `self.ReceiveTick`
  (params (DeltaSeconds :type "Float (single-precision)"))
  (`/Engine/EditorBlueprintResources/StandardMacros.Gate` true
    (:`Exit`
      (`self.K2_SetActorLocation` (`KismetMathLibrary.VInterpTo` (`self.K2_GetActorLocation`) (`self.K2_GetActorLocation`) DeltaSeconds 8.0)))))

(fn `UserConstructionScript`)