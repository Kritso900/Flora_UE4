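; ForSaleActor is a moveable object that displays a bloomed plant, presumably one put up for sale.
; A bound setup event receives the plant, picks the flower mesh by type and the material by colour, using per-type defaults or a debug "bad" material when colour is None.
; BeginPlay records the placement location and sizes the collision indicator and box from a small, medium or large scale through lookup maps.
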(event `Setup_Event` :!signature `self.Setup`
  (params (Plant :type "/Game/Characters/PlayerCharacter/InventoryItem_Struct Structure"))
  (bind _output_get (set `self.Plant` Plant))
  (switch `/Game/Characters/PlayerCharacter/PlantTypes_ENum` (`.PlantType_29_E290B51643956DE1EAD632A22DCE5ACD` (break `/Game/Characters/PlayerCharacter/InventoryItem_Struct` _output_get))
    (:`NewEnumerator0`
      (`StaticMeshComponent.SetStaticMesh` (`self.Flower`) "/Game/Meg_EnvironmentArt/Plants/Models/LavenderBloomed.LavenderBloomed"))
    (:`NewEnumerator1`
      (`StaticMeshComponent.SetStaticMesh` (`self.Flower`) "/Game/Meg_EnvironmentArt/Plants/Models/LilyBloomed.LilyBloomed"))
    (:`NewEnumerator2`
      (`StaticMeshComponent.SetStaticMesh` (`self.Flower`) "/Game/Meg_EnvironmentArt/Plants/Models/MiddlemistBloomed.MiddlemistBloomed"))
    (:`NewEnumerator3`
      (`StaticMeshComponent.SetStaticMesh` (`self.Flower`) "/Game/Meg_EnvironmentArt/Plants/Models/OrchidBloomed.OrchidBloomed"))
    (:`NewEnumerator4`
      (`StaticMeshComponent.SetStaticMesh` (`self.Flower`) "/Game/Meg_EnvironmentArt/Plants/Models/Rosebloomed.RoseBloomed"))
    (:`NewEnumerator5`
      (`StaticMeshComponent.SetStaticMesh` (`self.Flower`) "/Game/Meg_EnvironmentArt/Plants/Models/TulipBloomed.TulipBloomed")))
  ;[1 1 1] Sets up plant's material
  (switch `/Game/Characters/PlayerCharacter/PlantColours_Enum` (`.PlantColour_30_DCC94A0441A66B9EAC930D898107F0D4` (break `/Game/Characters/PlayerCharacter/InventoryItem_Struct` (`self.Plant`)))
    (:`NewEnumerator8`
      (switch `/Game/Characters/PlayerCharacter/PlantTypes_ENum` (`.PlantType_29_E290B51643956DE1EAD632A22DCE5ACD` (break `/Game/Characters/PlayerCharacter/InventoryItem_Struct` (`self.Plant`)))
        (:`NewEnumerator0`
          (`PrimitiveComponent.SetMaterial` (`self.Flower`) 0 "/Game/Meg_EnvironmentArt/Plants/Materials/PlantFlowerPurple_M.PlantFlowerPurple_M" :!label _label))
        (:`NewEnumerator1`
          (`PrimitiveComponent.SetMaterial` (`self.Flower`) 0 "/Game/Meg_EnvironmentArt/Plants/Materials/PlantFlowerBAD_M.PlantFlowerBAD_M" :!label _label_2) ; A debug material that only shows up\nif something has gone wrong
        )
        (:`NewEnumerator2`
          (`PrimitiveComponent.SetMaterial` (`self.Flower`) 0 "/Game/Meg_EnvironmentArt/Plants/Materials/PlantFlowerPink_M.PlantFlowerPink_M" :!label _label_3))
        (:`NewEnumerator3`
          (`PrimitiveComponent.SetMaterial` (`self.Flower`) 0 "/Game/Meg_EnvironmentArt/Plants/Materials/PlantFlowerWhite_M.PlantFlowerWhite_M" :!label _label_4))
        (:`NewEnumerator4`
          (goto _label_2))
        (:`NewEnumerator5`
          (goto _label_2))))
    (:`NewEnumerator0`
      (`PrimitiveComponent.SetMaterial` (`self.Flower`) 0 "/Game/Meg_EnvironmentArt/Plants/Materials/PlantFlowerBlack_M.PlantFlowerBlack_M"))
    (:`NewEnumerator1`
      (`PrimitiveComponent.SetMaterial` (`self.Flower`) 0 "/Game/Meg_EnvironmentArt/Plants/Materials/PlantFlowerBlue_M.PlantFlowerBlue_M"))
    (:`NewEnumerator2`
      (`PrimitiveComponent.SetMaterial` (`self.Flower`) 0 "/Game/Meg_EnvironmentArt/Plants/Materials/PlantFlowerOrange_M.PlantFlowerOrange_M"))
    (:`NewEnumerator3`
      (goto _label_3))
    (:`NewEnumerator5`
      (goto _label))
    (:`NewEnumerator4`
      (`PrimitiveComponent.SetMaterial` (`self.Flower`) 0 "/Game/Meg_EnvironmentArt/Plants/Materials/PlantFlowerRed_M.PlantFlowerRed_M"))
    (:`NewEnumerator6`
      (goto _label_4))
    (:`NewEnumerator7`
      (`PrimitiveComponent.SetMaterial` (`self.Flower`) 0 "/Game/Meg_EnvironmentArt/Plants/Materials/PlantFlowerYellow_M.PlantFlowerYellow_M"))))

(event `self.ReceiveBeginPlay`
  (add `self.Setup` (delegate `Setup_Event`))
  (set `self.Object is Held` false)
  (set `self.Placement Location` (`self.K2_GetActorLocation`))
  (switch `/Game/MoveableObjects/ObjectScale_ENum` (`self.Object scale ENum`)
    (:`NewEnumerator0`
      (set `self.Object Scale` 1))
    (:`NewEnumerator1`
      (set `self.Object Scale` 2))
    (:`NewEnumerator2`
      (set `self.Object Scale` 3)))
  (`SceneComponent.SetWorldScale3D` (`self.Collision Indicator`) (`BlueprintMapLibrary.Map_Find` (`self.Collision checker Scale`) (`self.Object Scale`)))
  (`BoxComponent.SetBoxExtent` (`self.Collision Box`) (`BlueprintMapLibrary.Map_Find` (`self.Collision box Scale`) (`self.Object Scale`)) false))

(event `self.ReceiveTick`
  (params (DeltaSeconds :type "Float (single-precision)"))
  (`|ExecutionSequence`))

(fn `UserConstructionScript`)