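; Medium moveable flower object that the player can pick up, rotate and place.
; A bound setup event picks the bloomed mesh and colour material from the plant's type and colour, with a debug material for invalid defaults.
; Pickup disables collision; when released, Tick eases it to the placement location and interpolates rotation between four steps.
; BeginPlay sizes collision components by object scale, and the collision indicator shows only in build mode.
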(event `Setup_Event` :!signature `self.Setup`
  (params (`Plant type` :type "/Game/Characters/PlayerCharacter/PlantTypes_ENum Enum" :default "NewEnumerator0") (`Plant colour` :type "/Game/Characters/PlayerCharacter/PlantColours_Enum Enum" :default "NewEnumerator8") (Plant :type "/Game/Characters/PlayerCharacter/InventoryItem_Struct Structure"))
  (bind _output_get (set `self.Plant` Plant))
  (switch `/Game/Characters/PlayerCharacter/PlantTypes_ENum` (`.PlantType_29_E290B51643956DE1EAD632A22DCE5ACD` (break `/Game/Characters/PlayerCharacter/InventoryItem_Struct` _output_get))
    (:`NewEnumerator0`
      (`StaticMeshComponent.SetStaticMesh` (`self.Flower`) "/Game/Meg_EnvironmentArt/Plants/Models/LavenderBloomed.LavenderBloomed"))
    (:`NewEnumerator1`
      (`StaticMeshComponent.SetStaticMesh` (`self.Flower`) "/Game/Meg_EnvironmentArt/Plants/Models/LilyBloomed.LilyBloomed"))
    (:`NewEnumerator2`
      (`StaticMeshComponent.SetStaticMesh` (`self.Flower`) "/Game/Meg_EnvironmentArt/Plants/Models/MiddlemistBloomed.MiddlemistBloomed"))
    (:`NewEnumerator3`
      (`StaticMeshComponent.SetStaticMesh` (`self.Flower`) "/Game/Meg_EnvironmentArt/Plants/Models/OrchidBloomed.OrchidBloomed"))
    (:`NewEnumerator4`
      (`StaticMeshComponent.SetStaticMesh` (`self.Flower`) "/Game/Meg_EnvironmentArt/Plants/Models/Rosebloomed.RoseBloomed"))
    (:`NewEnumerator5`
      (`StaticMeshComponent.SetStaticMesh` (`self.Flower`) "/Game/Meg_EnvironmentArt/Plants/Models/TulipBloomed.TulipBloomed")))
  ;[1 1 1] Sets up plant's material
  (switch `/Game/Characters/PlayerCharacter/PlantColours_Enum` (`.PlantColour_30_DCC94A0441A66B9EAC930D898107F0D4` (break `/Game/Characters/PlayerCharacter/InventoryItem_Struct` (`self.Plant`)))
    (:`NewEnumerator8`
      (switch `/Game/Characters/PlayerCharacter/PlantTypes_ENum` (`.PlantType_29_E290B51643956DE1EAD632A22DCE5ACD` (break `/Game/Characters/PlayerCharacter/InventoryItem_Struct` (`self.Plant`)))
        (:`NewEnumerator0`
          (`PrimitiveComponent.SetMaterial` (`self.Flower`) 0 "/Game/Meg_EnvironmentArt/Plants/Materials/PlantFlowerPurple_M.PlantFlowerPurple_M" :!label _label))
        (:`NewEnumerator1`
          (`PrimitiveComponent.SetMaterial` (`self.Flower`) 0 "/Game/Meg_EnvironmentArt/Plants/Materials/PlantFlowerBAD_M.PlantFlowerBAD_M" :!label _label_2) ; A debug material that only shows up\nif something has gone wrong
        )
        (:`NewEnumerator2`
          (`PrimitiveComponent.SetMaterial` (`self.Flower`) 0 "/Game/Meg_EnvironmentArt/Plants/Materials/PlantFlowerPink_M.PlantFlowerPink_M" :!label _label_3))
        (:`NewEnumerator3`
          (`PrimitiveComponent.SetMaterial` (`self.Flower`) 0 "/Game/Meg_EnvironmentArt/Plants/Materials/PlantFlowerWhite_M.PlantFlowerWhite_M" :!label _label_4))
        (:`NewEnumerator4`
          (goto _label_2))
        (:`NewEnumerator5`
          (goto _label_2))))
    (:`NewEnumerator0`
      (`PrimitiveComponent.SetMaterial` (`self.Flower`) 0 "/Game/Meg_EnvironmentArt/Plants/Materials/PlantFlowerBlack_M.PlantFlowerBlack_M"))
    (:`NewEnumerator1`
      (`PrimitiveComponent.SetMaterial` (`self.Flower`) 0 "/Game/Meg_EnvironmentArt/Plants/Materials/PlantFlowerBlue_M.PlantFlowerBlue_M"))
    (:`NewEnumerator2`
      (`PrimitiveComponent.SetMaterial` (`self.Flower`) 0 "/Game/Meg_EnvironmentArt/Plants/Materials/PlantFlowerOrange_M.PlantFlowerOrange_M"))
    (:`NewEnumerator3`
      (goto _label_3))
    (:`NewEnumerator5`
      (goto _label))
    (:`NewEnumerator4`
      (`PrimitiveComponent.SetMaterial` (`self.Flower`) 0 "/Game/Meg_EnvironmentArt/Plants/Materials/PlantFlowerRed_M.PlantFlowerRed_M"))
    (:`NewEnumerator6`
      (goto _label_4))
    (:`NewEnumerator7`
      (`PrimitiveComponent.SetMaterial` (`self.Flower`) 0 "/Game/Meg_EnvironmentArt/Plants/Materials/PlantFlowerYellow_M.PlantFlowerYellow_M"))))

(event `self.ReceiveBeginPlay`
  (add `self.Place Object` (delegate `Place Object_Event`))
  (add `self.Pickup Object` (delegate `Pickup Object_Event`))
  (add `self.Rotate Left` (delegate `Rotate Left_Event`))
  (add `self.Rotate Right` (delegate `Rotate Right_Event`))
  (add `self.Setup` (delegate `Setup_Event`))
  (set `self.Object is Held` false)
  (set `self.Placement Location` (`self.K2_GetActorLocation`))
  (switch `/Game/MoveableObjects/ObjectScale_ENum` (`self.Object scale ENum`)
    (:`NewEnumerator0`
      (set `self.Object Scale` 1))
    (:`NewEnumerator1`
      (set `self.Object Scale` 2))
    (:`NewEnumerator2`
      (set `self.Object Scale` 3)))
  (`SceneComponent.SetWorldScale3D` (`self.Collision Indicator`) (`BlueprintMapLibrary.Map_Find` (`self.Collision checker Scale`) (`self.Object Scale`)))
  (`BoxComponent.SetBoxExtent` (`self.Collision Box`) (`BlueprintMapLibrary.Map_Find` (`self.Collision box Scale`) (`self.Object Scale`)) false))

(event `Place Object_Event` :!signature `self.Place Object`
  (params (`Placement Location` :type "Vector Structure"))
  (set `self.Placement Location` `Placement Location`)
  (`PrimitiveComponent.SetCollisionEnabled` (`self.Collision Box`) "QueryAndPhysics")
  (set `self.Object is Held` false)
  (`PrimitiveComponent.SetMaterial` (`self.Collision Indicator`) 0 "/Game/MoveableObjects/CollisionOK_M.CollisionOK_M"))

(event `self.ReceiveTick`
  (params (DeltaSeconds :type "Float (single-precision)"))
  (bind _collision_indicator (`self.Collision Indicator`))
  (`|ExecutionSequence`
    (:`then_0`
      (if (not (`self.Object is Held`))
        (`self.K2_SetActorLocation` (`KismetMathLibrary.VInterpTo` (`self.K2_GetActorLocation`) (`self.Placement Location`) DeltaSeconds 12.0))))
    (:`then_1`
      (`self.K2_SetActorRotation` (`KismetMathLibrary.RInterpTo` (`self.K2_GetActorRotation`) (`|GetArrayItem` (`self.Rotations`) (`self.Target Rotation`)) DeltaSeconds 5.0))
      (`KismetSystemLibrary.Delay` 0.2)
      (bind _asplayer_character_bp (cast `/Game/Characters/PlayerCharacter/PlayerCharacter_BP` (`GameplayStatics.GetPlayerPawn` 0)))
      (if (`/Game/Characters/PlayerCharacter/PlayerCharacter_BP.Is Player in build mode` _asplayer_character_bp)
        (`SceneComponent.SetVisibility` _collision_indicator true false)
        (else
          (`SceneComponent.SetVisibility` _collision_indicator false false))))))

(event `Pickup Object_Event`
  (`PrimitiveComponent.SetCollisionEnabled` (`self.Collision Box`) "NoCollision")
  (set `self.Object is Held` true))

(event `Rotate Left_Event`
  (bind _target_rotation (`self.Target Rotation`))
  (if (`self.Object is Held`)
    (if (== _target_rotation 0)
      (set `self.Target Rotation` 3)
      (else
        (`/Engine/EditorBlueprintResources/StandardMacros.DecrementInt` _target_rotation)))))

(event `Rotate Right_Event`
  (bind _target_rotation (`self.Target Rotation`))
  (if (`self.Object is Held`)
    (if (== _target_rotation 3)
      (set `self.Target Rotation` 0)
      (else
        (`/Engine/EditorBlueprintResources/StandardMacros.IncrementInt` _target_rotation)))))

(fn `UserConstructionScript`)